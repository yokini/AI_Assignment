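; BP_Navlink is a smart nav link that makes AI characters jump to the link's destination.
; When an AI_Character reaches the link, it computes a ballistic launch velocity from the agent's location, the destination and a JumpDuration, then launches the character with full velocity override.
; CalculateVelocity solves projectile motion for that flight time, using a hardcoded gravity of 982 rather than the world setting.
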(event `self.ReceiveSmartLinkReached`
  (params (Agent :type "Actor Object Reference") (Destination :type "Vector Structure (by ref)"))
  (bind _asai_character (cast `/Game/GamePlay/Blueprints/AI_Character` Agent))
  (bind _velocity (`self. CalculateVelocity` (`self.JumpDuration`) Destination (`self.K2_GetActorLocation` _asai_character)))
  (`Character.LaunchCharacter` _asai_character _velocity true true))

(fn ` CalculateVelocity`
  (params (Duration :type "Float (double-precision)") (EndPoint :type "Vector Structure") (StartPoint :type "Vector Structure"))
  (returns (Velocity :type "Vector Structure"))
  (locals (L_Duration :type "Float (double-precision)"))
  (bind _l_duration (`local.L_Duration`))
  (set `local.L_Duration` Duration)
  (return (`KismetMathLibrary.MakeVector` (/ (- EndPoint_X StartPoint_X) _l_duration) (/ (- EndPoint_Y StartPoint_Y) _l_duration) (/ (- EndPoint_Z (+ StartPoint_Z (* (`KismetMathLibrary.Square` (`local.L_Duration`)) -0.5 982.0))) _l_duration))))

(fn `UserConstructionScript`)